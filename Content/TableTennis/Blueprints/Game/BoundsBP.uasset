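; BoundsBP is a table tennis boundary actor that tells the ball whether it is in or out of bounds.
; Overlaps on its InBounds and OutBounds components cast to BP_GrippableTennisBall and call the ball's matching InBounds or OutOfBounds function.
; The construction script scales both trigger components and the Cube from the Size and Height variables, keeping a fixed thickness for each.
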(event OnComponentBeginOverlap(InBounds)
  (params (OverlappedComponent :type Primitive%20Component%20Object%20Reference) (OtherActor :type Actor%20Object%20Reference) (OtherComp :type Primitive%20Component%20Object%20Reference) (OtherBodyIndex :type Integer) (bFromSweep :type Boolean) (SweepResult :type Hit%20Result%20Structure%20%28by%20ref%29))
  (bind _asbp_grippable_tennis_ball (Utilities|Casting|CastToBP_GrippableTennisBall OtherActor))
  (Default|InBounds _asbp_grippable_tennis_ball))

(event OnComponentBeginOverlap(OutBounds)
  (params (OverlappedComponent :type Primitive%20Component%20Object%20Reference) (OtherActor :type Actor%20Object%20Reference) (OtherComp :type Primitive%20Component%20Object%20Reference) (OtherBodyIndex :type Integer) (bFromSweep :type Boolean) (SweepResult :type Hit%20Result%20Structure%20%28by%20ref%29))
  (bind _asbp_grippable_tennis_ball (Utilities|Casting|CastToBP_GrippableTennisBall OtherActor))
  (Default|OutOfBounds _asbp_grippable_tennis_ball))

(event EventBeginPlay)

(event Collision|EventActorBeginOverlap
  (params (OtherActor :type Actor%20Object%20Reference)))

(event EventTick
  (params (DeltaSeconds :type Float%20%28single-precision%29)))

(fn ConstructionScript
  (bind _size (Variables|Default|GetSize))
  (bind _height (Variables|Default|GetHeight))
  (Transformation|SetRelativeScale3D (Variables|Default|GetOutBounds) (Math|Vector|MakeVector (* _size 1.5625) 0.5 (* _height 1.5625)))
  (Transformation|SetRelativeScale3D (Variables|Default|GetCube) (Math|Vector|MakeVector _size 0.25 _height)))