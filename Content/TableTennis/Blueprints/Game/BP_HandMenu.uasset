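; Hand menu actor for the table tennis game that floats a widget beside the player's left hand.
; Every Tick it offsets the widget from the hand toward and above along the hand-to-camera look-at axes, using MenuDistanceToCamera for both offsets.
; It then rotates the widget to face the player camera.
; CloseMenu destroys the actor.
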(event Custom|Close%20Menu
  (Actor|DestroyActor))

(event EventBeginPlay
  (|CallParentFunction) ; This node is disabled and will not be called.\nDrag off pins to build functionality.
)

(event Collision|EventActorBeginOverlap
  (params (OtherActor :type Actor%20Object%20Reference))
  (|CallParentFunction OtherActor) ; This node is disabled and will not be called.\nDrag off pins to build functionality.
)

(event EventTick
  (params (DeltaSeconds :type Float%20%28single-precision%29))
  (bind _returnvalue (Game|GetPlayerCameraManager 0))
  (bind _menudistancetocamera (Variables|Default|GetMenuDistanceToCamera))
  (bind _lefthandref (Variables|Default|GetLeftHandRef))
  (bind _returnvalue_2 (Camera|GetCameraLocation _returnvalue))
  (bind _returnvalue_3 (Transformation|GetWorldLocation _lefthandref))
  (bind _returnvalue_4 (Math|Rotator|FindLookatRotation _returnvalue_3 _returnvalue_2))
  (|CallParentFunction DeltaSeconds)
  (Transformation|SetWorldLocation (Variables|Default|GetWidget) (+ _returnvalue_3 (* (Math|Vector|GetForwardVector _returnvalue_4) _menudistancetocamera) (* (Math|Vector|GetUpVector _returnvalue_4) _menudistancetocamera)) false false)
  (Transformation|SetWorldRotation (Variables|Default|GetWidget) (Math|Rotator|FindLookatRotation (Transformation|GetWorldLocation (Variables|Default|GetWidget)) (Camera|GetCameraLocation (Game|GetPlayerCameraManager 0))) false false))

(fn ConstructionScript
  (|CallParentFunction))