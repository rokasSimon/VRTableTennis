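; Game mode for VR table tennis that gives each joining player an index.
; When a new player starts, it checks for the VR template player controller and writes a running counter into that player's BP_TennisPlayerState as PlayerIndex, then increments it.
; Other controller types only print a warning, whose text still says PostLogin.
; PostLogin itself is empty, and an older player-count-based assignment and a join message are left disconnected.
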(event EventPostLogin
  (params (NewPlayer :type Player%20Controller%20Object%20Reference)))

(event EventHandleStartingNewPlayer
  (params (NewPlayer :type Player%20Controller%20Object%20Reference))
  (bind _astemplate_vr_player_controller (Utilities|Casting|CastToTemplate_VR_Player_Controller NewPlayer)
    (:then
      (bind _asbp_tennis_player_state (Utilities|Casting|CastToBP_TennisPlayerState (Variables|/Script/Engine.Controller|GetPlayerState _astemplate_vr_player_controller)))
      (Variables|/Game/TableTennis/Blueprints/Game/BP_TennisPlayerState.BP_TennisPlayerState_C|SetPlayerIndex _asbp_tennis_player_state (Variables|Default|GetNextPlayerIndex))
      (Variables|Default|SetNextPlayerIndex (+ (Variables|Default|GetNextPlayerIndex) 1)))
    (:CastFailed
      (Development|PrintString "PostLogin: Not a Template_VR_Player_Controller"))))

(fn ConstructionScript
  (|CallParentFunction))